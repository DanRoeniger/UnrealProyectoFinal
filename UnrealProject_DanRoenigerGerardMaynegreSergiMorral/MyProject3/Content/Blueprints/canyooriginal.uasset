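; Cannon turret actor that tracks player pawn 0 and fires Balacanyo projectiles at it.
; Each Tick, constant-speed float interpolation turns the actor's yaw and pitches the Canyo component toward the player, with pitch moving much faster.
; When yaw is nearly aligned and the player is within Distancia, it calls Shoot.
; Shoot spawns the projectile along the barrel's forward vector, using DoOnce plus a RECARGA delay as the reload cooldown.
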(event Custom|shoot
  (bind _scene (Variables|Default|GetScene))
  (Utilities|FlowControl|DoOnce false :!label _label
    (:Completed
      (Game|SpawnActorfromClass "/Game/Blueprints/balacanyo.balacanyo_C" (Math|Transform|MakeTransform (Transformation|GetWorldLocation _scene) (Transformation|GetWorldRotation _scene)) "AlwaysSpawn" 0 (Math|Vector|GetForwardVector (Variables|Default|Getcanyo)) 5e+03 0)
      (Utilities|FlowControl|Delay (Variables|Default|GetRECARGA))
      (goto _label Reset))))

(event EventTick
  (params (DeltaSeconds :type Float%20%28single-precision%29))
  (bind _returnvalue (Game|Player|GetPlayerPawn 0))
  (bind _returnvalue_2 (Transformation|GetActorRotation))
  (bind _returnvalue_3 (Utilities|Time|GetWorldDeltaSeconds))
  (bind _canyo (Variables|Default|Getcanyo))
  (bind _returnvalue_4 (Transformation|GetActorLocation _returnvalue))
  (bind _returnvalue_5 (Transformation|GetWorldLocation _canyo))
  (bind _yaw (Math|Rotator|BreakRotator _returnvalue_2))
  (bind _returnvalue_6 (Math|Rotator|FindLookatRotation _returnvalue_5 _returnvalue_4))
  (bind (_roll _pitch _yaw_2) (Math|Rotator|BreakRotator _returnvalue_6))
  (bind _returnvalue_7 (Math|Interpolation|FInterptoConstant _yaw _yaw_2 _returnvalue_3 5e+01))
  (Transformation|SetActorRotation (Math|Rotator|MakeRotator 0.0 0.0 _returnvalue_7))
  (Transformation|SetWorldRotation (Variables|Default|Getcanyo) (Math|Rotator|MakeRotator 0.0 (Math|Interpolation|FInterptoConstant (.Pitch (Math|Rotator|BreakRotator (Transformation|GetWorldRotation (Variables|Default|Getcanyo)))) _pitch _returnvalue_3 1e+03) _returnvalue_7) false false)
  (if (Math|Float|NearlyEqual(Float) _yaw_2 _yaw 2.0)
    (if (>= (Variables|Default|Getdistancia) (Math|Vector|VectorLength (- (Transformation|GetActorLocation (Game|Player|GetPlayerPawn 0)) (Transformation|GetWorldLocation (Variables|Default|Getbasesm)))))
      (CallFunction|Shoot))))

(fn ConstructionScript)