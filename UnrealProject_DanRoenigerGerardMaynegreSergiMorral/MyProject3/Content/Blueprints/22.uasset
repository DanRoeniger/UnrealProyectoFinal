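; Configurable platform actor that can slide along X, spin its mesh or, in Muntanya mode, rotate its Scene1 component instead of sliding.
; The Segura flag picks a wood or transparent dynamic material, whose Brillo parameter follows Tocant every tick.
; Player overlap brightens a safe platform, while an unsafe one runs a timeline that drives Brillo and a text timer, then destroys the actor.
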(event EventBeginPlay
  (if (not (Variables|Default|Getmuntanya))
    (bind _newtrack_0 (Timeline|Timeline_0 Play)
      (:Update
        (Transformation|SetRelativeLocation (Variables|Default|GetStaticMesh) (Math|Vector|MakeVector (* _newtrack_0 (Variables|Default|Getoffsed)) 0.0 0.0) false false)
        (Components|Timeline|SetPlayRate (Variables|Default|GetTimeline_0) (/ 1.0 (Variables|Default|Getduracio)))))))

(event EventTick
  (params (DeltaSeconds :type Float%20%28single-precision%29))
  (Rendering|Material|SetScalarParameterValue (Variables|Default|GetNewVar_0) "Brillo" (Variables|Default|Gettocant) :!class /Script/Engine.MaterialInstanceDynamic)
  (if (Variables|Default|Getrotatori)
    (Transformation|SetRelativeRotation (Variables|Default|GetStaticMesh) (Math|Rotator|MakeRotator 0.0 0.0 (+ (.yaw (.rotation (Transformation|GetRelativeTransform (Variables|Default|GetStaticMesh)))) 1.0)) false false))
  (if (Variables|Default|Getmuntanya)
    (Transformation|SetRelativeRotation (Variables|Default|GetScene1) (Math|Rotator|MakeRotator 0.0 0.0 (+ (.yaw (.rotation (Transformation|GetRelativeTransform (Variables|Default|GetScene1)))) (Variables|Default|Getvelrotaciomuntanya))) false false)))

(event Collision|EventActorEndOverlap
  (params (OtherActor :type Actor%20Object%20Reference))
  (Utilities|Casting|CastToplayer OtherActor)
  (Variables|Default|Settocant 0.0))

(event Collision|EventActorBeginOverlap
  (params (OtherActor :type Actor%20Object%20Reference))
  (bind _tempstransp (Variables|Default|Gettempstransp))
  (Utilities|Casting|CastToplayer OtherActor)
  (if (Variables|Default|Getsegura)
    (Variables|Default|Settocant 1e+01)
    (else
      (bind _newtrack_2 (Timeline|Timeline_2 Play)
        (:Update
          (Variables|Default|Settocant _newtrack_2)
          (Rendering|Components|TextRender|SetText (Variables|Default|GetTextRender) (Utilities|Text|ToText(Float) (* _newtrack_2 _tempstransp) "HalfToEven"))
          (Components|Timeline|SetPlayRate (Variables|Default|GetTimeline_2) (/ 1.0 _tempstransp))
          (Rendering|SetVisibility (Variables|Default|GetTextRender) true false))
        (:Finished
          (Actor|DestroyActor))))))

(fn ConstructionScript
  (if (Variables|Default|Getsegura)
    (bind _returnvalue (Rendering|Material|CreateDynamicMaterialInstance "/Game/StarterContent/Materials/M_Wood_Oak.M_Wood_Oak" :!class /Script/Engine.KismetMaterialLibrary))
    (bind _output_get (Variables|Default|SetNewVar_0 _returnvalue))
    (Rendering|Material|SetMaterial (Variables|Default|GetStaticMesh) 0 _output_get)
    (else
      (bind _returnvalue_2 (Rendering|Material|CreateDynamicMaterialInstance "/Game/Blueprints/Materials/transp_Inst.transp_Inst" :!class /Script/Engine.KismetMaterialLibrary))
      (bind _output_get_2 (Variables|Default|SetNewVar_0 _returnvalue_2))
      (Rendering|Material|SetMaterial (Variables|Default|GetStaticMesh) 0 _output_get_2)
      (Variables|Default|Settocant 1.0))))