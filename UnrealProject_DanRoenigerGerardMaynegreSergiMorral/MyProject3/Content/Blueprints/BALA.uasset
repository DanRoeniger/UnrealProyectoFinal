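; BALA is a bullet actor that flies along its forward vector at constant speed and explodes on timeout or impact.
; Tick moves it without sweep, and BeginPlay destroys it with a fire-bomb explosion after a short delay.
; Overlap damages enemic1's Vida and sets its blackboard chase flag, or destroys a dron while the bullet survives.
; It ignores the player and explodes on any other actor.
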(event EventBeginPlay
  (Utilities|FlowControl|Delay 2.0)
  (Effects|SpawnEmitteratLocation "/Game/InfinityBladeEffects/Effects/FX_Monsters/FX_Monster_Gruntling/Bomber/P_FireBombExplosion.P_FireBombExplosion" (Transformation|GetActorLocation self))
  (Actor|DestroyActor))

(event Collision|EventActorBeginOverlap
  (params (OtherActor :type Actor%20Object%20Reference))
  (bind _self self)
  (bind _returnvalue (Transformation|GetActorLocation _self))
  (bind _asenemic_1 (Utilities|Casting|CastToenemic1 OtherActor)
    (:then
      (Variables|/Game/Blueprints/enemic1.enemic1_C|Setvida _asenemic_1 (- (Variables|/Game/Blueprints/enemic1.enemic1_C|Getvida _asenemic_1) 5.0))
      (Effects|SpawnEmitteratLocation "/Game/InfinityBladeEffects/Effects/FX_Monsters/FX_Monster_Gruntling/Bomber/P_FireBombExplosion.P_FireBombExplosion" _returnvalue)
      (AI|Components|Blackboard|SetValueasBool (AI|GetBlackboard _asenemic_1) (Utilities|Name|MakeLiteralName "Persiguiendo") true)
      (Actor|DestroyActor))
    (:CastFailed
      (bind _asenemicvolador (Utilities|Casting|CastTodron OtherActor)
        (:then
          (Effects|SpawnEmitteratLocation "/Game/InfinityBladeEffects/Effects/FX_Monsters/FX_Monster_Gruntling/Bomber/P_FireBombExplosion.P_FireBombExplosion" _returnvalue)
          (Actor|DestroyActor _asenemicvolador))
        (:CastFailed
          (Utilities|Casting|CastToplayer OtherActor
            (:CastFailed
              (Effects|SpawnEmitteratLocation "/Game/InfinityBladeEffects/Effects/FX_Monsters/FX_Monster_Gruntling/Bomber/P_FireBombExplosion.P_FireBombExplosion" _returnvalue)
              (Actor|DestroyActor))))))))

(event EventTick
  (params (DeltaSeconds :type Float%20%28single-precision%29))
  (bind _self self)
  (Transformation|SetActorLocation (+ (Transformation|GetActorLocation _self) (* (* (Math|Vector|GetForwardVector (Transformation|GetActorRotation _self)) 7e+02) (Utilities|Time|GetWorldDeltaSeconds))) false false))

(fn ConstructionScript)