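; Behavior tree service that tells an AI when the player is within hearing distance and hands it the player as a target while chasing.
; Each tick it writes the Escuchado blackboard bool from a fixed-radius distance check between the controlled pawn and the player pawn.
; While Persiguiendo is true, it sets Target to the player and stops the AI controller's current movement.
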(event EventTick
  (params (OwnerActor :type Actor%20Object%20Reference) (DeltaSeconds :type Float%20%28single-precision%29))
  (bind _returnvalue (Game|Player|GetPlayerPawn 0))
  (bind _asaicontroller (Utilities|Casting|CastToAIController OwnerActor))
  (Class|BTFunctionLibrary|SetBlackboardValueasBool (Variables|Default|Getescuchado) (<= (Math|Vector|VectorLength (- (Transformation|GetActorLocation (Pawn|GetControlledPawn _asaicontroller)) (Transformation|GetActorLocation _returnvalue))) 2e+03))
  (if (Class|BTFunctionLibrary|GetBlackboardValueasBool (Variables|Default|GetPersiguiendo))
    (Class|BTFunctionLibrary|SetBlackboardValueasObject (Variables|Default|GetTarget) _returnvalue)
    (AI|Navigation|StopMovement _asaicontroller)))