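; Speed boost pickup actor that the player collects by walking into it.
; On overlap with the player, it sets the Boostveloctat flag in the game instance's Inventory, plays a sound at the world origin and destroys itself.
; Tick polls the same flag and jumps into that sound-and-destroy chain, so any copy present while the boost is owned removes itself, also playing the sound.
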(event Collision|EventActorBeginOverlap
  (params (OtherActor :type Actor%20Object%20Reference))
  (Utilities|Casting|CastToplayer OtherActor)
  (bind _asmy_game_instance_bp (Utilities|Casting|CastToMyGameInstanceBP (Game|GetGameInstance)))
  (Utilities|Struct|SetmembersinSInventory (Variables|/Game/Blueprints/MyGameInstanceBP.MyGameInstanceBP_C|GetInventory _asmy_game_instance_bp) true)
  (Audio|PlaySoundatLocation "/Game/SaveLoadGame/Sounds/correct-ding_Auto9.correct-ding" "0, 0, 0")
  (Actor|DestroyActor))

(event EventTick
  (params (DeltaSeconds :type Float%20%28single-precision%29))
  (bind _asmy_game_instance_bp (Utilities|Casting|CastToMyGameInstanceBP (Game|GetGameInstance)))
  (if (.boostveloctat (Utilities|Struct|BreakSInventory (Variables|/Game/Blueprints/MyGameInstanceBP.MyGameInstanceBP_C|GetInventory _asmy_game_instance_bp)))
    (Audio|PlaySoundatLocation "/Game/SaveLoadGame/Sounds/correct-ding_Auto9.correct-ding" "0, 0, 0")
    (Actor|DestroyActor)))

(fn ConstructionScript)