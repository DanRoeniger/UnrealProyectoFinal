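; Cannonball projectile that launches its static mesh on BeginPlay with an impulse from its direction and power variables.
; On overlap it spawns an explosion and destroys itself, ignoring the cannon class and other cannonballs.
; Player hits remove life through the GameInstance, while enemy hits subtract directly from that enemy's Vida.
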(event EventBeginPlay
  (Physics|AddImpulse (Variables|Default|GetStaticMesh) (* (Variables|Default|Getdirection) (Variables|Default|Getpotenci)) "None" true))

(event Collision|EventActorBeginOverlap
  (params (OtherActor :type Actor%20Object%20Reference))
  (bind _asplayer (Utilities|Casting|CastToplayer OtherActor)
    (:then
      (Effects|SpawnEmitteratLocation "/Game/StarterContent/Particles/P_Explosion.P_Explosion" (Transformation|GetActorLocation _asplayer))
      (bind _asmy_game_instance_bp (Utilities|Casting|CastToMyGameInstanceBP (Game|GetGameInstance)))
      (Default|Treurevida _asmy_game_instance_bp 5.0)
      (Actor|DestroyActor))
    (:CastFailed
      (bind _asenemic_1 (Utilities|Casting|CastToenemic1 OtherActor)
        (:then
          (Effects|SpawnEmitteratLocation "/Game/StarterContent/Particles/P_Explosion.P_Explosion" (Transformation|GetActorLocation _asenemic_1))
          (Variables|/Game/Blueprints/enemic1.enemic1_C|Setvida _asenemic_1 (- (Variables|/Game/Blueprints/enemic1.enemic1_C|Getvida _asenemic_1) 5.0))
          (Actor|DestroyActor))
        (:CastFailed
          (Utilities|Casting|CastTocanyooriginal OtherActor
            (:CastFailed
              (Utilities|Casting|CastTobalacanyo OtherActor
                (:CastFailed
                  (Effects|SpawnEmitteratLocation "/Game/StarterContent/Particles/P_Explosion.P_Explosion" (Transformation|GetActorLocation OtherActor))
                  (Actor|DestroyActor))))))))))

(fn ConstructionScript)