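; Drone actor that faces the player and explodes on overlap, removing health when it hits the player.
; Each tick it sets the Perseguir (chase) flag from whether the player is within Rango and rotates toward them; no movement is scripted here.
; Any overlap spawns an explosion and destroys the drone, with player hits first calling Treurevida on the game instance.
; The construction script applies a dynamic material instance to the mesh.
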(event EventTick
  (params (DeltaSeconds :type Float%20%28single-precision%29))
  (bind _returnvalue (Game|Player|GetPlayerPawn 0))
  (bind _self self)
  (bind _returnvalue_2 (Transformation|GetActorLocation _returnvalue))
  (bind _returnvalue_3 (Transformation|GetActorLocation _self))
  (Variables|Default|Setperseguir (>= (Variables|Default|Getrango) (Math|Vector|VectorLength (- _returnvalue_2 _returnvalue_3))))
  (Transformation|SetActorRotation (Math|Rotator|FindLookatRotation _returnvalue_3 _returnvalue_2)))

(event Collision|EventActorBeginOverlap
  (params (OtherActor :type Actor%20Object%20Reference))
  (bind _asplayer (Utilities|Casting|CastToplayer OtherActor)
    (:then
      (Effects|SpawnEmitteratLocation "/Game/StarterContent/Particles/P_Explosion.P_Explosion" (Transformation|GetActorLocation _asplayer))
      (bind _asmy_game_instance_bp (Utilities|Casting|CastToMyGameInstanceBP (Game|GetGameInstance)))
      (Default|Treurevida _asmy_game_instance_bp 1e+01))
    (:CastFailed
      (Effects|SpawnEmitteratLocation "/Game/StarterContent/Particles/P_Explosion.P_Explosion" (Transformation|GetWorldLocation (Variables|Default|GetStaticMesh)))))
  (Actor|DestroyActor))

(fn ConstructionScript
  (bind _returnvalue (Rendering|Material|CreateDynamicMaterialInstance "/Game/Blueprints/Materials/MAT6_Inst.MAT6_Inst" :!class /Script/Engine.KismetMaterialLibrary))
  (bind _output_get (Variables|Default|SetNewVar_0 _returnvalue))
  (Rendering|Material|SetMaterial (Variables|Default|GetStaticMesh) 0 _output_get))