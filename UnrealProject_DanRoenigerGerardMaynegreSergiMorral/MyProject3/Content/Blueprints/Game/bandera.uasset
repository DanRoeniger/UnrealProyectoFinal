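; Flag pickup actor (bandera) that the player collects by touching it.
; On overlap with a player, it calls Conseguirbandera on the game instance with 1, sets Agafat, plays a fabric sound at world origin, hides itself and destroys its Box component.
; While Agafat is true, Tick repeats the hide and Box destruction every frame.
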(event EventBeginPlay)

(event Collision|EventActorBeginOverlap
  (params (OtherActor :type Actor%20Object%20Reference))
  (Utilities|Casting|CastToplayer OtherActor)
  (bind _asmy_game_instance_bp (Utilities|Casting|CastToMyGameInstanceBP (Game|GetGameInstance)))
  (Default|Conseguirbandera _asmy_game_instance_bp 1)
  (Variables|Default|Setagafat true)
  (Audio|PlaySoundatLocation "/Game/SaveLoadGame/Sounds/220936__nebulousflynn__folding-fabric-sheets_Auto9.220936__nebulousflynn__folding-fabric-sheets" "0, 0, 0")
  (Rendering|SetActorHiddenInGame true)
  (Components|DestroyComponent (Variables|Default|GetBox)))

(event EventTick
  (params (DeltaSeconds :type Float%20%28single-precision%29))
  (if (Variables|Default|Getagafat)
    (Rendering|SetActorHiddenInGame true)
    (Components|DestroyComponent (Variables|Default|GetBox))))

(fn ConstructionScript)