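; Game instance that holds the player's inventory (flags, health, jetpack, speed boost) and handles death and save/load.
; Helpers add or spend flags and subtract health; at zero, Matar ragdolls the player, with its reset-and-reload code left unreachable.
; Saving writes inventory, position, Barratemps and flag pickup states, matched by actor index, to one slot.
; Loading calls OpenLevel for ProyectoFinal, then restores that data immediately in the same call.
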(fn Conseguirbandera
  (params (Numbanderes :type Integer))
  (Utilities|Struct|SetmembersinSInventory (Variables|Default|GetInventory) (+ Numbanderes (.Numbanderes (Utilities|Struct|BreakSInventory (Variables|Default|GetInventory)))))
  (return))

(fn Consumirbanderes
  (params (Numbanderes :type Integer))
  (if (<= Numbanderes (.Numbanderes (Utilities|Struct|BreakSInventory (Variables|Default|GetInventory))))
    (Utilities|Struct|SetmembersinSInventory (Variables|Default|GetInventory) (- (.Numbanderes (Utilities|Struct|BreakSInventory (Variables|Default|GetInventory))) Numbanderes))
    (return true)
    (else
      (return false))))

(fn Treurevida
  (params (vidaquetreu :type Float%20%28single-precision%29))
  (bind _inventory (Variables|Default|GetInventory))
  (bind _vida (Utilities|Struct|BreakSInventory _inventory))
  (bind _returnvalue (- _vida vidaquetreu))
  (bind _returnvalue_2 (Math|Float|Clamp(Float) _returnvalue 0.0 1e+02))
  (if (>= 0.0 _returnvalue)
    (Utilities|Struct|SetmembersinSInventory (Variables|Default|GetInventory) _returnvalue_2)
    (CallFunction|Matar)
    (return)
    (else
      (Utilities|Struct|SetmembersinSInventory _inventory _returnvalue_2)
      (return))))

(fn Matar
  (bind _asplayer (Utilities|Casting|CastToplayer (Game|Player|GetPlayerPawn 0)))
  (Physics|SetSimulatePhysics (Variables|/Script/Engine.Character|GetMesh _asplayer) true)
  (Components|DestroyComponent (Variables|/Script/Engine.Character|GetCapsuleComponent _asplayer)))

(fn Cargarpartida
  (bind _returnvalue (Game|GetPlayerCharacter 0))
  (Game|OpenLevel(byName) "ProyectoFinal")
  (bind _asmy_game_instance_bp (Utilities|Casting|CastToMyGameInstanceBP (Game|GetGameInstance)))
  (bind _returnvalue_2 (SaveGame|DoesSaveGameExist "Ranura1"))
  (if _returnvalue_2
    (bind _returnvalue_3 (SaveGame|LoadGamefromSlot "Ranura1"))
    (Variables|Default|Setsavegame _returnvalue_3)
    (bind _asplayer (Utilities|Casting|CastToplayer _returnvalue))
    (bind _asguardar_partida_classe (Utilities|Casting|CastToGuardarPartidaClasse _returnvalue_3))
    (Transformation|SetActorLocation _returnvalue (Variables|/Game/SaveLoadGame/GuardarPartidaClasse.GuardarPartidaClasse_C|GetPosicionJugador _asguardar_partida_classe) false false)
    (bind _output_get (Variables|/Game/Blueprints/player.player_C|Setbarratemps _asplayer (Variables|/Game/SaveLoadGame/GuardarPartidaClasse.GuardarPartidaClasse_C|GetStopTime _asguardar_partida_classe)))
    (Development|PrintString (Utilities|String|ToString(Float) (Variables|/Game/Blueprints/player.player_C|Getbarratemps _asplayer)))
    (if (> (Variables|/Game/SaveLoadGame/GuardarPartidaClasse.GuardarPartidaClasse_C|GetVida _asguardar_partida_classe) 0.0)
      (Variables|/Game/SaveLoadGame/GuardarPartidaClasse.GuardarPartidaClasse_C|SetVida _asguardar_partida_classe (Variables|/Game/SaveLoadGame/GuardarPartidaClasse.GuardarPartidaClasse_C|GetVida _asguardar_partida_classe))
      (else
        (Variables|/Game/SaveLoadGame/GuardarPartidaClasse.GuardarPartidaClasse_C|SetVida _asguardar_partida_classe 1e+02)))
    (bind _outactors (Actor|GetAllActorsOfClass "/Game/Blueprints/Game/bandera.bandera_C"))
    (for (_array_element _array_index) (Variables|/Game/SaveLoadGame/GuardarPartidaClasse.GuardarPartidaClasse_C|Getbanderesagafades _asguardar_partida_classe)
      (Variables|/Game/Blueprints/Game/bandera.bandera_C|Setagafat (Utilities|Array|Get(acopy) _outactors _array_index) _array_element)
      (Utilities|Struct|SetmembersinSInventory (Variables|MyGameInstanceBP_C|GetInventory _asmy_game_instance_bp) (Variables|/Game/SaveLoadGame/GuardarPartidaClasse.GuardarPartidaClasse_C|GetNumBanderes _asguardar_partida_classe) 0 (Variables|/Game/SaveLoadGame/GuardarPartidaClasse.GuardarPartidaClasse_C|GetVida _asguardar_partida_classe) (Variables|/Game/SaveLoadGame/GuardarPartidaClasse.GuardarPartidaClasse_C|GetVidaTotal _asguardar_partida_classe) (Variables|/Game/SaveLoadGame/GuardarPartidaClasse.GuardarPartidaClasse_C|GetJetpack _asguardar_partida_classe) (Variables|/Game/SaveLoadGame/GuardarPartidaClasse.GuardarPartidaClasse_C|GetBoostVel _asguardar_partida_classe)))
    (else
      (Development|PrintString "NO HI HA"))))

(fn Guardarjoc
  (bind _asmy_game_instance_bp (Utilities|Casting|CastToMyGameInstanceBP (Game|GetGameInstance)))
  (bind _returnvalue (SaveGame|CreateSaveGameObject "/Game/SaveLoadGame/GuardarPartidaClasse.GuardarPartidaClasse_C"))
  (Variables|Default|Setsavegame _returnvalue)
  (bind _asplayer (Utilities|Casting|CastToplayer (Game|GetPlayerCharacter 0)))
  (bind _asguardar_partida_classe (Utilities|Casting|CastToGuardarPartidaClasse _returnvalue))
  (Variables|/Game/SaveLoadGame/GuardarPartidaClasse.GuardarPartidaClasse_C|SetStopTime _asguardar_partida_classe (Variables|/Game/Blueprints/player.player_C|Getbarratemps _asplayer))
  (Variables|/Game/SaveLoadGame/GuardarPartidaClasse.GuardarPartidaClasse_C|SetNumBanderes _asguardar_partida_classe (.Numbanderes (Utilities|Struct|BreakSInventory (Variables|MyGameInstanceBP_C|GetInventory _asmy_game_instance_bp))))
  (Variables|/Game/SaveLoadGame/GuardarPartidaClasse.GuardarPartidaClasse_C|SetPosicionJugador _asguardar_partida_classe (Transformation|GetWorldLocation (Variables|/Script/Engine.Character|GetCapsuleComponent _asplayer)))
  (Variables|/Game/SaveLoadGame/GuardarPartidaClasse.GuardarPartidaClasse_C|SetVida _asguardar_partida_classe (.vida (Utilities|Struct|BreakSInventory (Variables|MyGameInstanceBP_C|GetInventory _asmy_game_instance_bp))))
  (Variables|/Game/SaveLoadGame/GuardarPartidaClasse.GuardarPartidaClasse_C|SetVidaTotal _asguardar_partida_classe (.vidatotal (Utilities|Struct|BreakSInventory (Variables|MyGameInstanceBP_C|GetInventory _asmy_game_instance_bp))))
  (Variables|/Game/SaveLoadGame/GuardarPartidaClasse.GuardarPartidaClasse_C|SetJetpack _asguardar_partida_classe (.jetpack (Utilities|Struct|BreakSInventory (Variables|MyGameInstanceBP_C|GetInventory _asmy_game_instance_bp))))
  (Variables|/Game/SaveLoadGame/GuardarPartidaClasse.GuardarPartidaClasse_C|SetBoostVel _asguardar_partida_classe (.boostveloctat (Utilities|Struct|BreakSInventory (Variables|MyGameInstanceBP_C|GetInventory _asmy_game_instance_bp))))
  (bind _outactors (Actor|GetAllActorsOfClass "/Game/Blueprints/Game/bandera.bandera_C"))
  (for (_array_element _array_index) _outactors
    (Utilities|Array|Insert (Variables|/Game/SaveLoadGame/GuardarPartidaClasse.GuardarPartidaClasse_C|Getbanderesagafades _asguardar_partida_classe) (Variables|/Game/Blueprints/Game/bandera.bandera_C|Getagafat _array_element) _array_index)
    (SaveGame|SaveGametoSlot _returnvalue "Ranura1")))