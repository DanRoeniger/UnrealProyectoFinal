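; Jetpack pickup actor that boosts the player's jumping and records the item in the game instance's inventory.
; On player overlap it sets the Jetpack flag, raises air control, jump hold time and max jump count, plays a sound and destroys itself.
; Tick checks that flag and, if already set, reapplies the same boosts with the sound and removes the pickup without an overlap.
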(event EventBeginPlay)

(event Collision|EventActorBeginOverlap
  (params (OtherActor :type Actor%20Object%20Reference))
  (bind _asplayer (Utilities|Casting|CastToplayer OtherActor))
  (bind _asmy_game_instance_bp (Utilities|Casting|CastToMyGameInstanceBP (Game|GetGameInstance)))
  (Utilities|Struct|SetmembersinSInventory (Variables|/Game/Blueprints/MyGameInstanceBP.MyGameInstanceBP_C|GetInventory _asmy_game_instance_bp) true)
  (Variables|/Script/Engine.CharacterMovementComponent|SetAirControl (Variables|/Script/Engine.Character|GetCharacterMovement _asplayer) 1.0)
  (Variables|/Script/Engine.Character|SetJumpMaxHoldTime (Game|GetPlayerCharacter 0) 5.0)
  (Variables|/Script/Engine.Character|SetJumpMaxCount _asplayer 3)
  (Audio|PlaySoundatLocation "/Game/SaveLoadGame/Sounds/correct-ding_Auto9.correct-ding" "0, 0, 0")
  (Actor|DestroyActor))

(event EventTick
  (params (DeltaSeconds :type Float%20%28single-precision%29))
  (bind _asmy_game_instance_bp (Utilities|Casting|CastToMyGameInstanceBP (Game|GetGameInstance)))
  (if (.jetpack (Utilities|Struct|BreakSInventory (Variables|/Game/Blueprints/MyGameInstanceBP.MyGameInstanceBP_C|GetInventory _asmy_game_instance_bp)))
    (bind _asplayer (Utilities|Casting|CastToplayer (Game|Player|GetPlayerPawn 0)))
    (Variables|/Script/Engine.CharacterMovementComponent|SetAirControl (Variables|/Script/Engine.Character|GetCharacterMovement _asplayer) 1.0)
    (Variables|/Script/Engine.Character|SetJumpMaxHoldTime (Game|GetPlayerCharacter 0) 5.0)
    (Variables|/Script/Engine.Character|SetJumpMaxCount _asplayer 3)
    (Audio|PlaySoundatLocation "/Game/SaveLoadGame/Sounds/correct-ding_Auto9.correct-ding" "0, 0, 0")
    (Actor|DestroyActor)))

(fn ConstructionScript)