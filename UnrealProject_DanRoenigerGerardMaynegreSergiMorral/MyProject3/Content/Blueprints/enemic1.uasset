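; Enemy AI pawn that chases the player and explodes on contact, calling Treurevida on the game instance to take life from the player.
; PawnSensing sets the Persiguiendo (chasing) blackboard flag on sight.
; Tick updates a health bar widget from Vida/Salutmaxima and yaws it toward the player.
; At zero Vida, the mesh ragdolls and the capsule and widget are destroyed.
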(event OnSeePawn(PawnSensing)
  (params (Pawn :type Pawn%20Object%20Reference))
  (AI|Components|Blackboard|SetValueasBool (AI|GetBlackboard self) (Utilities|Name|MakeLiteralName "Persiguiendo") true))

(event EventBeginPlay)

(event Collision|EventActorBeginOverlap
  (params (OtherActor :type Actor%20Object%20Reference))
  (Utilities|Casting|CastToplayer OtherActor)
  (bind _asmy_game_instance_bp (Utilities|Casting|CastToMyGameInstanceBP (Game|GetGameInstance)))
  (Default|Treurevida _asmy_game_instance_bp 5e+01)
  (Effects|SpawnEmitteratLocation "/Game/StarterContent/Particles/P_Explosion.P_Explosion" (Transformation|GetActorLocation OtherActor))
  (Actor|DestroyActor))

(event EventTick
  (params (DeltaSeconds :type Float%20%28single-precision%29))
  (bind _vida (Variables|Default|Getvida))
  (bind _widget (Variables|Default|GetWidget))
  (if (<= _vida 0.0)
    (Physics|SetSimulatePhysics (Variables|Character|GetMesh) true)
    (Components|DestroyComponent (Variables|Collision|GetCapsuleComponent))
    (Components|DestroyComponent (Variables|Default|GetWidget))
    (else
      (bind _assalutenemics (Utilities|Casting|CastTosalutenemics (UserInterface|GetUserWidgetObject (Variables|Default|GetWidget))))
      (Progress|SetPercent (Variables|/Game/Blueprints/huds/salutenemics.salutenemics_C|GetProgressBar_112 _assalutenemics) (/ _vida (Variables|Default|Getsalutmaxima)))
      (Transformation|SetWorldRotation _widget (Math|Rotator|MakeRotator 0.0 0.0 (.Yaw (Math|Rotator|BreakRotator (Math|Rotator|FindLookatRotation (Transformation|GetWorldLocation _widget) (Transformation|GetActorLocation (Game|Player|GetPlayerPawn 0)))))) false false))))

(fn ConstructionScript)